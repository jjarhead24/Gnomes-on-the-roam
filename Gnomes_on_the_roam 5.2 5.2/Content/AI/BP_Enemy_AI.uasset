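; BP_Enemy_AI is an enemy that chases the player once seen and can be killed.
; PawnSensing sets CanSeePlayer, which is never cleared here, and starts a follow event that uses AI MoveTo toward player 0.
; Reaching the player toggles CanAttack around a cooldown delay, though no attack is performed in this graph.
; Interact subtracts incoming damage from Health and destroys the actor when none remains.
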(event `self.PawnSensing.OnSeePawn`
  (params (Pawn :type "Pawn Object Reference"))
  (set `self.CanSeePlayer` true)
  (`self.follow_player`))

(event `follow_player`
  (set `self.CanAttack` true)
  (if (`self.CanSeePlayer`)
    (`|AIMoveTo` self (0.0 0.0 0.0) (`GameplayStatics.GetPlayerCharacter` 0)
      (:`OnSuccess`
        (if (`self.CanAttack`)
          (set `self.CanAttack` false)
          (`KismetSystemLibrary.Delay` 2.0)
          (set `self.CanAttack` true))))))

(event `/Game/BP_Interface.interact`
  (params (damage :type "Float (double-precision)"))
  (bind _output_get (set `self.Health` (- (`self.Health`) damage)))
  (if (not (> _output_get 0.0))
    (`self.K2_DestroyActor`)))

(fn `UserConstructionScript`)