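; BP_enemy_character is a gnome enemy whose health comes from the game instance at BeginPlay.
; A Walking timeline, started at BeginPlay, drives its max walk speed.
; Damage lowers health and awards the player points per hit, while a special sentinel damage value kills instantly.
; Death awards points and a kill, spawns BP_GnomeShatter, calls GnomeCheck, decrements the game instance's gnome counters and destroys the actor.
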(event `/Game/BP_Interface_damage.Damage`
  (params (Damage_amount :type "Float (double-precision)"))
  (bind _as_bp_game_instance (`self.As BP Game Instance`))
  (bind _asbp_first_person_character (cast `/Game/FirstPerson/Blueprints/BP_FirstPersonCharacter` (`GameplayStatics.GetPlayerCharacter` 0)))
  (if (== Damage_amount -10.0)
    (set `/Game/FirstPerson/Blueprints/BP_FirstPersonCharacter.Points` (+ (`/Game/FirstPerson/Blueprints/BP_FirstPersonCharacter.Points` _asbp_first_person_character) (`self.pointer_per_kill`)) _asbp_first_person_character :!label _label)
    (set `/Game/FirstPerson/Blueprints/BP_FirstPersonCharacter.Kills` (+ (`/Game/FirstPerson/Blueprints/BP_FirstPersonCharacter.Kills` _asbp_first_person_character) 1) _asbp_first_person_character)
    (`CharacterMovementComponent.DisableMovement` (`self.CharacterMovement`))
    (`|SpawnActorFromClass` "/Game/BluePrints/BP_GnomeShatter.BP_GnomeShatter_C" (`SceneComponent.K2_GetComponentToWorld` (`self.Mesh`)) "Undefined" "MultiplyWithRoot" null null)
    (`/Game/BP_GameInstance.GnomeCheck` _as_bp_game_instance)
    (set `/Game/BP_GameInstance.GnomesLeftInRound` (- (`/Game/BP_GameInstance.GnomesLeftInRound` _as_bp_game_instance) 1) _as_bp_game_instance)
    (set `/Game/BP_GameInstance.GnomesOnMap` (- (`/Game/BP_GameInstance.GnomesOnMap` _as_bp_game_instance) 1.0) _as_bp_game_instance)
    (`self.K2_DestroyActor`)
    (else
      (bind _output_get (set `self.Health` (- (`self.Health`) Damage_amount)))
      (set `/Game/FirstPerson/Blueprints/BP_FirstPersonCharacter.Points` (+ (`/Game/FirstPerson/Blueprints/BP_FirstPersonCharacter.Points` _asbp_first_person_character) 10) _asbp_first_person_character)
      (if (not (> _output_get 0.0))
        (goto _label)))))

(event `self.ReceiveBeginPlay`
  (bind _asbp_game_instance (cast `/Game/BP_GameInstance` (`GameplayStatics.GetGameInstance`)))
  (set `self.As BP Game Instance` _asbp_game_instance)
  (set `self.Health` (`/Game/BP_GameInstance.GnomeHealth` _asbp_game_instance))
  (bind (_direction _walking_speed) (`Timeline|Walking`)
    (:`Update`
      (set `CharacterMovementComponent.MaxWalkSpeed` _walking_speed (`self.CharacterMovement`)))))

(fn `UserConstructionScript`)