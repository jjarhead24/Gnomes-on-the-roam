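; BP_Planter is an interactable planter that grows the player's held seed, one plant until removed, and updates PlantsOnMap, calling OpenSunny at four.
; Planting swaps linked cable materials and starts that plant's behavior.
; Venus damages overlapping enemies on a looping timer; Cactus periodically targets a random enemy, swings its arm and spawns a velocity-led projectile.
; Datura, Sunflower and Rose only set flags and borrow the Venus model as a placeholder.
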(event `/Game/BP_Interface.interact`
  (params (damage :type "Float (double-precision)") (remove_plant :type Boolean))
  (`|ExecutionSequence`
    (:`then_0`
      (if (> damage 0.0)
        _
        (elif remove_plant
          ;[1 1 1] remove the plant
          (`SceneComponent.SetVisibility` (`self.Venus`) false false)
          (`SceneComponent.SetVisibility` (`self.Cactus_Arm`) false false)
          (`SceneComponent.SetVisibility` (`self.Cactus`) false false)
          (`KismetSystemLibrary.K2_ClearAndInvalidateTimerHandle` (`self.VenusTimer`))
          (`KismetSystemLibrary.K2_ClearAndInvalidateTimerHandle` (`self.CactusTimeRef`))
          (set `self.VenusEnabled` false)
          (set `self.CactusEnabled` false)
          (set `self.RoseEnabled` false)
          (bind _asbp_first_person_character (cast `/Game/FirstPerson/Blueprints/BP_FirstPersonCharacter` (`GameplayStatics.GetPlayerCharacter` 0)))
          (set `/Game/FirstPerson/Blueprints/BP_FirstPersonCharacter.Plants_On_map` (- (`/Game/FirstPerson/Blueprints/BP_FirstPersonCharacter.Plants_On_map` _asbp_first_person_character) 1) _asbp_first_person_character)
          (`KismetSystemLibrary.K2_ClearAndInvalidateTimerHandle` (`self.VenusTimer`))
          (goto _label :!via `Reset`)
          (else
            (`/Engine/EditorBlueprintResources/StandardMacros.DoOnce` false :!label _label
              (:`Completed`
                (bind _asbp_first_person_character_2 (cast `/Game/FirstPerson/Blueprints/BP_FirstPersonCharacter` (`GameplayStatics.GetPlayerCharacter` 0)))
                (set `/Game/FirstPerson/Blueprints/BP_FirstPersonCharacter.Plants_On_map` (+ (`/Game/FirstPerson/Blueprints/BP_FirstPersonCharacter.Plants_On_map` _asbp_first_person_character_2) 1) _asbp_first_person_character_2)
                (bind _heldseed (`/Game/FirstPerson/Blueprints/BP_FirstPersonCharacter.HeldSeed` _asbp_first_person_character_2))
                (if (== _heldseed "Venus")
                  (`SceneComponent.SetVisibility` (`self.Venus`) true false)
                  (set `self.VenusEnabled` true)
                  (set `self.CurrentPlant` _heldseed)
                  (`self.Change cable Mat`)
                  (`self.venusActive`)
                  (elif (== _heldseed "Datura")
                    (`SceneComponent.SetVisibility` (`self.Venus`) true false)
                    (set `self.DaturaEnabled` true)
                    (set `self.CurrentPlant` _heldseed)
                    (`self.Change cable Mat`)
                    (elif (== _heldseed "Sunflower")
                      (`SceneComponent.SetVisibility` (`self.Venus`) true false)
                      (set `self.SunflowerEnabled` true)
                      (set `self.CurrentPlant` _heldseed)
                      (`self.Change cable Mat`)
                      (elif (== _heldseed "Cactus")
                        (`SceneComponent.SetVisibility` (`self.Cactus`) true true)
                        (set `self.CactusEnabled` true)
                        (set `self.CurrentPlant` _heldseed)
                        (`self.ShootStarter`)
                        (`self.Change cable Mat`)
                        (elif (== _heldseed "Rose")
                          (`SceneComponent.SetVisibility` (`self.Venus`) true false)
                          (set `self.RoseEnabled` true)
                          (set `self.CurrentPlant` _heldseed)
                          (`self.Change cable Mat`)
                          (else
                            (goto _label :!via `Reset`)))))))))))))
    (:`then_1`
      (bind _asbp_first_person_character_3 (cast `/Game/FirstPerson/Blueprints/BP_FirstPersonCharacter` (`GameplayStatics.GetPlayerCharacter` 0)))
      (if (== (`/Game/FirstPerson/Blueprints/BP_FirstPersonCharacter.Plants_On_map` _asbp_first_person_character_3) 4)
        (`/Game/FirstPerson/Blueprints/BP_FirstPersonCharacter.Open Sunny` _asbp_first_person_character_3)))))

(event `venusActive`
  (bind _returnvalue (`KismetSystemLibrary.K2_SetTimerDelegate` (delegate `Venus Killer`) (`self.VenusAttackTime`) true))
  (set `self.VenusTimer` _returnvalue))

(event `Venus Killer`
  (for _array_element (`PrimitiveComponent.GetOverlappingActors` (`self.Venus_DeathBox`) "/Game/AI/BP_enemy_character.BP_enemy_character_C")
    (message `/Game/BP_Interface_damage.Damage` _array_element -10.0)))

(event `ShootStarter`
  (bind _returnvalue (`KismetSystemLibrary.K2_SetTimerDelegate` (delegate `CactusShoot`) (`self.CactusShootTime`) true))
  (set `self.CactusTimeRef` _returnvalue)
  (bind _output_get (set `self.ArmStartAngle` (`SceneComponent.RelativeRotation` (`self.Rotate point`)))))

(event `CactusShoot`
  (bind _gnomeref (`self.GnomeRef`))
  (bind _returnvalue (`SceneComponent.K2_GetComponentLocation` (`self.ProjSpawnPos`)))
  (bind _returnvalue_2 (`self.K2_GetActorLocation` _gnomeref))
  (bind _outitem (`KismetArrayLibrary.Array_Random` (`PrimitiveComponent.GetOverlappingActors` (`self.CactusDeathBox`) "/Game/AI/BP_enemy_character.BP_enemy_character_C")))
  (bind _returnvalue_3 (`KismetMathLibrary.FindLookAtRotation` _returnvalue _returnvalue_2))
  (`/Engine/EditorBlueprintResources/StandardMacros.IsValid` _outitem
    (:`Is Valid`
      (set `self.GnomeRef` _outitem)
      (`SceneComponent.K2_SetWorldRotation` (`self.ProjSpawnPos`) _returnvalue_3 false false)
      (`SceneComponent.K2_SetWorldRotation` (`self.Cactus`) (`KismetMathLibrary.MakeRotator` 0.0 0.0 (.yaw (* _returnvalue_3 -1.0))) false false)
      (bind (_direction _newtrack_1) (`Timeline|Timeline` :!via `PlayFromStart`)
        (:`Update`
          (`SceneComponent.K2_SetRelativeRotation` (`self.Rotate point`) (`KismetMathLibrary.RLerp` (stale `ShootStarter` _output_get) (struct :`Yaw` 30.0 :`Roll` 45.0) _newtrack_1) false false))
        (:`event`
          (`/Engine/EditorBlueprintResources/StandardMacros.IsValid` _gnomeref
            (:`Is Valid`
              (`|SpawnActorFromClass` "/Game/FirstPerson/Blueprints/BP_FirstPersonProjectile.BP_FirstPersonProjectile_C" (`KismetMathLibrary.MakeTransform` _returnvalue (`KismetMathLibrary.FindLookAtRotation` _returnvalue (+ _returnvalue_2 (* (`self.GetVelocity` _gnomeref) (/ (`self.GetDistanceTo` _gnomeref) 3000.0))))) "AlwaysSpawn" "MultiplyWithRoot" null null))))))))

(fn `Change cable Mat`
  (`PrimitiveComponent.SetMaterial` (`CableActor.CableComponent` (`self.CableRef3`)) 0 "/Game/Materials/Power_Lines/m_Power_lines.m_Power_lines")
  (`PrimitiveComponent.SetMaterial` (`CableActor.CableComponent` (`self.CableRef2`)) 0 "/Game/Materials/Power_Lines/m_Power_lines.m_Power_lines")
  (`PrimitiveComponent.SetMaterial` (`CableActor.CableComponent` (`self.CableRef1`)) 0 "/Game/Materials/Power_Lines/m_Power_lines.m_Power_lines")
  (`PrimitiveComponent.SetMaterial` (`CableActor.CableComponent` (`self.CableRef`)) 0 "/Game/Materials/Power_Lines/m_Power_lines.m_Power_lines")
  (`PrimitiveComponent.SetMaterial` (`CableActor.CableComponent` (`self.CableRef4`)) 0 "/Game/Materials/Power_Lines/m_Power_lines.m_Power_lines")
  (`PrimitiveComponent.SetMaterial` (`CableActor.CableComponent` (`self.CableRef5`)) 0 "/Game/Materials/Power_Lines/m_Power_lines.m_Power_lines"))

(fn `UserConstructionScript`)