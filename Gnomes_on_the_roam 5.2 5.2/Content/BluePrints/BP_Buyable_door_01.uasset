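; A buyable double-door that the player opens by spending points, with its cost shown on a text render.
; On Interact it deducts the cost from the first-person character's Points and plays purchase and gate sounds, or a can't-afford sound otherwise.
; A purchase sets Door1 in the game instance, saves, and swings two cubes open via a timeline.
; The checks that destroy an already-bought door are unconnected and never run.
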(event `self.ReceiveBeginPlay`
  (`TextRenderComponent.K2_SetText` (`self.TextRender`) (`KismetTextLibrary.Conv_IntToText` (`self.Door_cost`))))

(event `self.ReceiveTick`
  (params (DeltaSeconds :type "Float (single-precision)")))

(event `/Game/BP_Interface.interact`
  (params (damage :type "Float (double-precision)") (remove_plant :type Boolean))
  (bind _returnvalue (`SceneComponent.K2_GetComponentLocation` (`self.DefaultSceneRoot`)))
  (bind _asbp_first_person_character (cast `/Game/FirstPerson/Blueprints/BP_FirstPersonCharacter` (`GameplayStatics.GetPlayerCharacter` 0)))
  (bind _returnvalue_2 (- (`/Game/FirstPerson/Blueprints/BP_FirstPersonCharacter.Points` _asbp_first_person_character) (`self.Door_cost`)))
  (if (>= _returnvalue_2 0)
    (set `/Game/FirstPerson/Blueprints/BP_FirstPersonCharacter.Points` _returnvalue_2 _asbp_first_person_character)
    (`GameplayStatics.PlaySoundAtLocation` "/Game/Audio/Purchase.Purchase" _returnvalue (struct) 1.0 1.0 0.0 null null null null)
    (bind _asbp_game_instance (cast `/Game/BP_GameInstance` (`GameplayStatics.GetGameInstance`)))
    (set `/Game/BP_GameInstance.Door_1` true _asbp_game_instance)
    (bind _asbp_game_instance_2 (cast `/Game/BP_GameInstance` (`GameplayStatics.GetGameInstance`)))
    (`/Game/BP_GameInstance.Save Game` _asbp_game_instance_2)
    (`GameplayStatics.PlaySoundAtLocation` "/Game/Audio/gate.gate" (`SceneComponent.K2_GetComponentLocation` (`self.DefaultSceneRoot`)) (struct) 1.0 1.0 3.0 null null null null)
    (bind (_direction _door) (`Timeline|open door`)
      (:`Update`
        (`SceneComponent.K2_SetRelativeRotation` (`self.Cube2`) (`KismetMathLibrary.RLerp` (struct) (struct :`Yaw` 90.0) _door) false false)
        (`SceneComponent.K2_SetRelativeRotation` (`self.Cube1`) (`KismetMathLibrary.RLerp` (struct) (struct :`Yaw` -90.0) _door) false false)))
    (else
      (`GameplayStatics.PlaySoundAtLocation` "/Game/Audio/Cant_Afford.Cant_Afford" _returnvalue (struct) 1.0 1.0 0.0 null null null null))))

(fn `UserConstructionScript`)