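; BP_seedbox is a seed stall where the player spends points to get a seed of the configured type.
; The construction script uses SeedType to show the Venus or Cactus component and set the matching stall material.
; On Interact, it checks the first-person character's Points against Price, deducts the cost, plays a purchase sound at the stall, and sets the character's HeldSeed to SeedType.
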(event `/Game/BP_Interface.interact`
  (params (damage :type "Float (double-precision)") (remove_plant :type Boolean))
  (bind _price (`self.Price`))
  (bind _asbp_first_person_character (cast `/Game/FirstPerson/Blueprints/BP_FirstPersonCharacter` (`GameplayStatics.GetPlayerCharacter` 0)))
  (bind _points (`/Game/FirstPerson/Blueprints/BP_FirstPersonCharacter.Points` _asbp_first_person_character))
  (if (>= _points _price)
    (set `/Game/FirstPerson/Blueprints/BP_FirstPersonCharacter.Points` (- _points _price) _asbp_first_person_character)
    (`GameplayStatics.PlaySoundAtLocation` "/Game/Audio/Purchase.Purchase" (`SceneComponent.K2_GetComponentLocation` (`self.SeedStall`)) (struct) 1.0 1.0 0.0 null null null null)
    (set `/Game/FirstPerson/Blueprints/BP_FirstPersonCharacter.HeldSeed` (`self.SeedType`) _asbp_first_person_character)))

(fn `UserConstructionScript`
  (if (== (`self.SeedType`) "Venus")
    (`SceneComponent.SetVisibility` (`self.Venus`) true false)
    (`PrimitiveComponent.SetMaterial` (`self.SeedStall`) 0 "/Game/Materials/Seed_Stalls/Venus_Fly_TRap/M_Seed_Venus.M_Seed_Venus")
    (elif (== (`self.SeedType`) "Cactus")
      (`SceneComponent.SetVisibility` (`self.Cactus`) true false)
      (`PrimitiveComponent.SetMaterial` (`self.SeedStall`) 0 "/Game/Materials/Seed_Stalls/Cacus/M_SS_Cactus.M_SS_Cactus"))))