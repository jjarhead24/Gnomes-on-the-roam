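; BP_GnomeGate is a gate that swings open for BP_enemy_character actors entering its Box trigger and closes once none remain.
; An enemy overlap plays the Open timeline, rotating RotatePoint from its current rotation to EndRote.
; Any overlap, even before the enemy cast, starts a looping three-second timer that checks the box.
; When it finds no enemies, a second timeline rotates the gate back and clears the timer.
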(event `self.Box.OnComponentBeginOverlap`
  (params (OverlappedComponent :type "PrimitiveComponent Object Reference") (OtherActor :type "Actor Object Reference") (OtherComp :type "PrimitiveComponent Object Reference") (OtherBodyIndex :type Integer) (bFromSweep :type Boolean) (SweepResult :type "HitResult Structure (by ref)"))
  (bind _returnvalue (`KismetSystemLibrary.K2_SetTimerDelegate` (delegate `door close`) 3.0 true))
  (set `self.door handle` _returnvalue)
  (cast `/Game/AI/BP_enemy_character` OtherActor)
  (bind _output_get (set `self.Start Rote` (`SceneComponent.RelativeRotation` (`self.rotate point`))))
  (bind (_direction _newtrack_0) (`Timeline|open` :!via `PlayFromStart`)
    (:`Update`
      (`SceneComponent.K2_SetRelativeRotation` (`self.rotate point`) (`KismetMathLibrary.RLerp` _output_get (`self.end rote`) _newtrack_0) false false))))

(event `door close`
  (if (`KismetArrayLibrary.Array_IsEmpty` (`PrimitiveComponent.GetOverlappingActors` (`self.Box`) "/Game/AI/BP_enemy_character.BP_enemy_character_C"))
    (bind (_direction _newtrack_0) (`Timeline|Timeline` :!via `PlayFromStart`)
      (:`Update`
        (`SceneComponent.K2_SetRelativeRotation` (`self.rotate point`) (`KismetMathLibrary.RLerp` (struct :`Yaw` 90.0) (struct) _newtrack_0) false false)
        (`KismetSystemLibrary.K2_ClearAndInvalidateTimerHandle` (`self.door handle`))))))

(fn `UserConstructionScript`)