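; BP_Sunny is an interactable actor that plays Sunny's one-shot upgrade animation while moving a Pistol component.
; On Interact, the MoveGun timeline raises the pistol, then after a fixed delay a second timeline lowers it.
; Both timelines lerp from the pistol's current relative transform toward a small Z offset, so movement compounds per update rather than using fixed endpoints.
; No upgrade logic is present; the sequence is purely visual.
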(event `/Game/BP_Interface.interact`
  (params (damage :type "Float (double-precision)") (remove_plant :type Boolean))
  (bind _pistol (`self.Pistol`))
  (bind _pistol_2 (`self.Pistol`))
  (bind _returnvalue_location (`KismetMathLibrary.BreakTransform` (`SceneComponent.GetRelativeTransform` _pistol_2)))
  (bind _returnvalue_location_2 (`KismetMathLibrary.BreakTransform` (`SceneComponent.GetRelativeTransform` _pistol)))
  (`SkeletalMeshComponent.PlayAnimation` (`self.Sunny`) "/Game/models/Sunny/SunnyUpgrade_Anim.SunnyUpgrade_Anim" false)
  (bind (_direction _gun) (`Timeline|move gun`)
    (:`Update`
      (`SceneComponent.K2_SetRelativeTransform` (`self.Pistol`) (`KismetMathLibrary.TLerp` (`SceneComponent.GetRelativeTransform` _pistol_2) (`KismetMathLibrary.Conv_VectorToTransform` (+ _returnvalue_location (0.0 0.0 3.5))) _gun) false false))
    (:`Finished`
      (`KismetSystemLibrary.Delay` 11.0)
      (bind (_direction_2 _gundown) (`Timeline|Timeline`)
        (:`Update`
          (`SceneComponent.K2_SetRelativeTransform` (`self.Pistol`) (`KismetMathLibrary.TLerp` (`SceneComponent.GetRelativeTransform` _pistol) (`KismetMathLibrary.Conv_VectorToTransform` (+ _returnvalue_location_2 (0.0 0.0 -3.5))) _gundown) false false))))))

(fn `UserConstructionScript`)