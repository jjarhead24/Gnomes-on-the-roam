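; BP_EletricArcs is an actor that draws an electric arc with a Niagara effect between start and end components.
; The construction script passes the End component's world location to the effect as its BeamEnd parameter.
; A DeleteNiagra event destroys the effect and a Cube component.
; Movement logic that would offset Start and End is left unconnected and never runs.
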(event `self.ReceiveBeginPlay`)

(event `/Game/BP_Interface_Eletric.DeleteNiagra`
  (`ActorComponent.K2_DestroyComponent` (`self.Eletric`))
  (`ActorComponent.K2_DestroyComponent` (`self.Cube`)))

(fn `UserConstructionScript`
  (`FXSystemComponent.SetVectorParameter` (`self.Eletric`) "BeamEnd" (`SceneComponent.K2_GetComponentLocation` (`self.End`))))