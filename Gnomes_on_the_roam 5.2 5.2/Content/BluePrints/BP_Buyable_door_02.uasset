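; BP_Buyable_door_02 is a door the player unlocks by spending points.
; On Interact, it deducts DoorCost from the first-person character's Points if affordable, sets the Door2 flag on BP_GameInstance, saves the game and destroys itself.
; BeginPlay and Tick both check that Door2 flag and destroy the door when it is already set, with Tick polling every frame.
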(event `self.ReceiveBeginPlay`
  (bind _asbp_game_instance (cast `/Game/BP_GameInstance` (`GameplayStatics.GetGameInstance`)))
  (if (`/Game/BP_GameInstance.Door_2` _asbp_game_instance)
    (`self.K2_DestroyActor`)))

(event `self.ReceiveTick`
  (params (DeltaSeconds :type "Float (single-precision)"))
  (bind _asbp_game_instance (cast `/Game/BP_GameInstance` (`GameplayStatics.GetGameInstance`)))
  (if (`/Game/BP_GameInstance.Door_2` _asbp_game_instance)
    (`self.K2_DestroyActor`)))

(event `/Game/BP_Interface.interact`
  (bind _asbp_first_person_character (cast `/Game/FirstPerson/Blueprints/BP_FirstPersonCharacter` (`GameplayStatics.GetPlayerCharacter` 0)))
  (bind _returnvalue (- (`/Game/FirstPerson/Blueprints/BP_FirstPersonCharacter.Points` _asbp_first_person_character) (`self.Door_cost`)))
  (if (>= _returnvalue 0)
    (set `/Game/FirstPerson/Blueprints/BP_FirstPersonCharacter.Points` _returnvalue _asbp_first_person_character)
    (bind _asbp_game_instance (cast `/Game/BP_GameInstance` (`GameplayStatics.GetGameInstance`)))
    (set `/Game/BP_GameInstance.Door_2` true _asbp_game_instance)
    (bind _asbp_game_instance_2 (cast `/Game/BP_GameInstance` (`GameplayStatics.GetGameInstance`)))
    (`/Game/BP_GameInstance.Save Game` _asbp_game_instance_2)
    (`self.K2_DestroyActor`)))

(fn `UserConstructionScript`)